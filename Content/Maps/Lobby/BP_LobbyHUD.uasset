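; Lobby HUD that shows the WBP_Lobby widget and keeps its player info and player list up to date.
; On BeginPlay it caches the owning BP_LobbyPlayerController, creates the widget and fills it with the controller's current data.
; It then binds to the controller's update delegates, so each change is pushed to the widget by event rather than polled.
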(event `self.ReceiveBeginPlay`
  (bind _player_controller (`self.Player Controller`))
  (`|ExecutionSequence`
    (:`then_0`
      ;[1 1 1] 初期化
      (bind _asbp_lobby_player_controller (cast `/Game/Maps/Lobby/BP_LobbyPlayerController` (`self.GetOwningPlayerController`)))
      (set `self.Player Controller` _asbp_lobby_player_controller))
    (:`then_1`
      ;[1 1 1] Widget作成
      (bind _returnvalue (`|CreateWidget` "/Game/Maps/Lobby/Widget/WBP_Lobby.WBP_Lobby_C" _player_controller))
      (bind _output_get (set `self.WBP` _returnvalue))
      (`UserWidget.AddToViewport` _output_get 0)
      (`/Game/Maps/Lobby/Widget/WBP_Lobby.SetPlayerInfo` (`self.WBP`) (`/Game/Maps/Lobby/BP_LobbyPlayerController.PlayerInfo` _player_controller))
      (`/Game/Maps/Lobby/Widget/WBP_Lobby.SetPlayerList` (`self.WBP`) (`/Game/Maps/Lobby/BP_LobbyPlayerController.PlayerList` _player_controller)))
    (:`then_2`
      ;[1 1 1] デリゲート登録
      (add `/Game/Maps/Lobby/BP_LobbyPlayerController.OnUpdatePlayerInfo` (`self.Player Controller`) (delegate `OnUpdatePlayerInfo`))
      (add `/Game/Maps/Lobby/BP_LobbyPlayerController.OnUpdatePlayerList` (`self.Player Controller`) (delegate `OnUpdatePlayerList`)))))

(event `OnUpdatePlayerInfo`
  ;[1 1 1] デリゲート登録
  (`/Game/Maps/Lobby/Widget/WBP_Lobby.SetPlayerInfo` (`self.WBP`) (`/Game/Maps/Lobby/BP_LobbyPlayerController.PlayerInfo` (`self.Player Controller`))))

(event `OnUpdatePlayerList`
  ;[1 1 1] デリゲート登録
  (`/Game/Maps/Lobby/Widget/WBP_Lobby.SetPlayerList` (`self.WBP`) (`/Game/Maps/Lobby/BP_LobbyPlayerController.PlayerList` (`self.Player Controller`))))

(fn `UserConstructionScript`)