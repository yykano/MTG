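; Lobby game mode that maintains the list of connected players and shares it with every lobby player controller.
; Logins arriving before BeginPlay are queued and processed afterwards, avoiding problems such as Characters not yet being spawned.
; Each login records ID, name and host status (local controller), then UpdatePlayerList copies the list to all controllers.
; Non-host logouts rebuild and redistribute the list; host logouts are ignored because clients also change level.
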(event `self.ReceiveBeginPlay`
  (bind _beforebeginplayloginplayers (`self.BeforeBeginPlayLoginPlayers`))
  ;[1 1 1] BeginPlay
  (`KismetSystemLibrary.PrintString` "GameMode: Event BeginPlay")
  (set `self.IsBeginPlayed` true)
  (for _array_element _beforebeginplayloginplayers
    (`/Engine/EditorBlueprintResources/StandardMacros.IsValid` _array_element
      (:`Is Valid`
        (`self.OnPostLogin` _array_element))))
  (`KismetArrayLibrary.Array_Clear` _beforebeginplayloginplayers))

(event `self.K2_PostLogin`
  (params (NewPlayer :type "PlayerController Object Reference"))
  ;[1 1 1] ログイン
  (if (`self.IsBeginPlayed`)
    (`self.OnPostLogin` NewPlayer)
    (else
      (`KismetArrayLibrary.Array_Add` (`self.BeforeBeginPlayLoginPlayers`) NewPlayer))))

(event `OnPostLogin`
  (params (NewPlayer :type "PlayerController Object Reference"))
  ;[1 1 1] ログイン処理(BeginPlay前に実行するとCharacterが生成されていなかったり不都合が多いため、BeginPlay後に実行できるようにしておく)
  (bind _asbp_lobby_player_controller (cast `/Game/Maps/Lobby/BP_LobbyPlayerController` NewPlayer))
  (`KismetArrayLibrary.Array_Add` (`self.PlayerConttollerList`) _asbp_lobby_player_controller)
  (bind _playerstate (`Controller.PlayerState` _asbp_lobby_player_controller))
  (bind _mtplayerinfo (make `MTPlayerInfo` (`PlayerState.PlayerId` _playerstate) (`PlayerState.GetPlayerName` _playerstate) (`Controller.IsLocalController` _asbp_lobby_player_controller)))
  (`KismetArrayLibrary.Array_Add` (`self.PlayerInfoList`) _mtplayerinfo)
  (set `/Game/Maps/Lobby/BP_LobbyPlayerController.PlayerInfo` _mtplayerinfo _asbp_lobby_player_controller)
  (`self.UpdatePlayerList`)
  (bind (_playerid _playername) (break `MTPlayerInfo` _mtplayerinfo))
  (`KismetSystemLibrary.PrintString` (`KismetTextLibrary.Conv_TextToString` (`|FormatText` "Player Login: {PlayerName} ({PlayerID})" _playername _playerid))))

(event `self.K2_OnLogout`
  (params (ExitingController :type "Controller Object Reference"))
  ;[1 1 1] ログアウト
  (if (not (`Controller.IsLocalController` ExitingController))
    (bind _asbp_lobby_player_controller (cast `/Game/Maps/Lobby/BP_LobbyPlayerController` ExitingController))
    ;;[1 1 1] 新規配列を用意
    (`KismetArrayLibrary.Array_RemoveItem` (`self.PlayerConttollerList`) _asbp_lobby_player_controller)
    (`KismetArrayLibrary.Array_Clear` (`self.PlayerInfoList_new`))
    ;;[1 1 1] ログアウトしたプレイヤー以外の情報を新規配列に追加
    (for _array_element (`self.PlayerInfoList`)
      (if (!= (`.PlayerId` (break `MTPlayerInfo` _array_element)) (`PlayerState.PlayerId` (`Controller.PlayerState` _asbp_lobby_player_controller)))
        (`KismetArrayLibrary.Array_Add` (`self.PlayerInfoList_new`) _array_element)))
    ;;[1 1 1] 配列を更新して通知イベント実行
    (set `self.PlayerInfoList` (`self.PlayerInfoList_new`))
    (`self.UpdatePlayerList`)))

(fn `UpdatePlayerList`
  (for _array_element (`self.PlayerConttollerList`)
    (bind _asbp_lobby_player_controller (cast `/Game/Maps/Lobby/BP_LobbyPlayerController` _array_element))
    (set `/Game/Maps/Lobby/BP_LobbyPlayerController.PlayerList` (`self.PlayerInfoList`) _asbp_lobby_player_controller)))

(fn `UserConstructionScript`)